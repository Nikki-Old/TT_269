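; Main game mode Blueprint that sets up save data when play begins.
; On BeginPlay it asks the SaveGameSubsystem to load the "Test" slot, or creates a new SaveGameMain in that slot if loading fails.
; Either result is cast to SaveGameMain and registered with the subsystem as the current save object.
; The slot name is hard-coded.
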(event EventBeginPlay
  (bind _returnvalue (Subsystems|GetSaveGameSubsystem))
  (|CallParentFunction)
  (bind (_savegameobject _returnvalue_2) (Class|SaveGameSubsystem|LoadSaveGame (Subsystems|GetSaveGameSubsystem) "Test"))
  (if _returnvalue_2
    (bind _assave_game_main (Utilities|Casting|CastToSaveGameMain _savegameobject))
    (Class|SaveGameSubsystem|SetCurrentSaveGameObject (Subsystems|GetSaveGameSubsystem) "Test" _assave_game_main)
    (else
      (bind (_savegameobject_2 _returnvalue_3) (Class|SaveGameSubsystem|CreateNewSaveGame _returnvalue "Test" "/Script/TT_269.SaveGameMain"))
      (if _returnvalue_3
        (bind _assave_game_main_2 (Utilities|Casting|CastToSaveGameMain _savegameobject_2))
        (Class|SaveGameSubsystem|SetCurrentSaveGameObject _returnvalue "Test" _assave_game_main_2)))))

(fn ConstructionScript)
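; Main HUD Blueprint that manages showing and hiding the player's inventory widget.
; ShowInventoryWidget lazily creates WBP_PlayerInventory on first use, passing it the InventoryComponent found on the owning player's pawn, then adds it to the viewport.
; The cached widget is then toggled between Visible and Collapsed, and IsShowInventoryWidget reports whether it is currently shown.
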(event EventBeginPlay)

(event Collision|EventActorBeginOverlap
  (params (OtherActor :type Actor%20Object%20Reference)))

(event EventTick
  (params (DeltaSeconds :type Float%20%28single-precision%29)))

(fn ConstructionScript)

(fn IsShowInventoryWidget
  (bind _inventorywidget (Variables|Default|GetInventoryWidget)
    (:then
      (return (Utilities|Select :Index (Widget|GetVisibility _inventorywidget) :Visible true :Collapsed false :Hidden false :HitTestInvisible true :SelfHitTestInvisible true)))
    (:else)))

(fn ShowInventoryWidget
  (params (bIsShow :type Boolean))
  (Variables|Default|GetInventoryWidget
    (:then
      _)
    (:else
      (bind _playerowner (Variables|Default|GetPlayerOwner)
        (:then
          (bind _output_get (LocalVariables|SetOwnerInventoryComponent_Local (Actor|GetComponentbyClass (Pawn|GetControlledPawn _playerowner) "/Script/TT_269.InventoryComponent")))
          (Utilities|IsValid _output_get
            (:Is%20Valid
              (bind _returnvalue (UserInterface|CreateWidget "/Game/TT_269/UI/Inventory/WBP_PlayerInventory.WBP_PlayerInventory_C" (Variables|Default|GetPlayerOwner) (LocalVariables|GetOwnerInventoryComponent_Local)))
              (bind _output_get_2 (Variables|Default|SetInventoryWidget _returnvalue))
              (UserInterface|Viewport|AddtoViewport _output_get_2 0))))
        (:else))))
  (Widget|SetVisibility (Variables|Default|GetInventoryWidget) (select bIsShow "Visible" "Collapsed")))
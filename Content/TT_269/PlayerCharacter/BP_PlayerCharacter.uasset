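; Player character Blueprint that handles movement, interaction, weapon combat, first aid kits, HUD widgets and save/load input.
; WeaponInventory slot changes drive SpawnWeapon, which replaces the socket-attached weapon, binds its fire and reload events and broadcasts animation updates.
; Reload waits for the montage to complete when one exists, then moves inventory ammo into the weapon.
; SaveGameActor callbacks store and respawn the weapon, while LoadPlayerInformation restores health and inventory.
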(event OnLoadGameData(SaveGameActor)
  ;[1 1 1] SaveGameActor:
  (Utilities|FlowControl|Sequence
    (:then_0
      (Weapon|SpawnWeapon (Variables|Weapon|GetSaveWeaponInfo)))
    (:then_1
      (Class|WeaponInventoryComponent|SetCurrentWeaponInfobySlotType (Variables|Default|GetWeaponInventory) (Class|WeaponInventoryComponent|GetCurrentWeaponInfoSlot (Variables|Default|GetWeaponInventory)) true))))

(event OnSaveGameData(SaveGameActor)
  ;[1 1 1] SaveGameActor:
  (Utilities|FlowControl|Sequence
    (:then_0
      ;;[1 1 1] Save WeaponInfo:
      (bind _currentweapon (Variables|Weapon|GetCurrentWeapon)
        (:then
          (Variables|Weapon|SetSaveWeaponInfo (Class|WeaponMain|GetWeaponActorInfo _currentweapon)))
        (:else)))))

(event Custom|PlayFireMontage_Event
  (params (AnimFireChar :type Anim%20Montage%20Object%20Reference))
  ;[1 1 1] Play anim montage:
  (Utilities|FlowControl|Sequence
    (:then_0
      (Weapon|SetCurrnetWeaponAmmoQuantity))
    (:then_1
      (Utilities|IsValid AnimFireChar
        (:Is%20Valid
          (Animation|Montage|PlayMontage (Variables|Character|GetMesh) AnimFireChar))))))

(event Custom|PlayReloadAnim_Event
  (params (AnimReloadChar :type Anim%20Montage%20Object%20Reference))
  ;[1 1 1] Play anim montage:
  (Utilities|IsValid AnimReloadChar
    (:Is%20Valid
      (Animation|Montage|PlayMontage (Variables|Character|GetMesh) AnimReloadChar
        (:OnCompleted
          (Weapon|Reload))))))

(event Input|EnhancedActionEvents|EnhancedInputActionIA_Move
  (params (ActionValue :type Vector%202D%20Structure) (ElapsedSeconds :type Float%20%28double-precision%29) (TriggeredSeconds :type Float%20%28double-precision%29) (InputAction :type Input%20Action%20Object%20Reference :default "/Game/TT_269/Core/Inputs/InputActions/IA_Move.IA_Move"))
  ;[1 1 1] Inputs:
  ;;[1 1 1] Movement input:
  (Class|PlayerCharacter|MovetoForward (.x ActionValue))
  (Class|PlayerCharacter|MovetoRight (.y ActionValue)))

(event Input|EnhancedActionEvents|EnhancedInputActionIA_Interact
  (params (ActionValue :type Boolean) (ElapsedSeconds :type Float%20%28double-precision%29) (TriggeredSeconds :type Float%20%28double-precision%29) (InputAction :type Input%20Action%20Object%20Reference :default "/Game/TT_269/Core/Inputs/InputActions/IA_Interact.IA_Interact"))
  (bind _interactsphere (Variables|Default|GetInteractSphere))
  (bind _returnvalue (Class|InteractSphereComponent|GetCurrentInteractTarget _interactsphere))
  ;[1 1 1] Inputs:
  ;;[1 1 1] Interact input:
  (:Started
    (Utilities|IsValid _returnvalue
      (:Is%20Valid
        (Class|InteractInterface|StartInteract(Message) _returnvalue self)))))

(event Input|EnhancedActionEvents|EnhancedInputActionIA_Inventory
  (params (ActionValue :type Boolean) (ElapsedSeconds :type Float%20%28double-precision%29) (TriggeredSeconds :type Float%20%28double-precision%29) (InputAction :type Input%20Action%20Object%20Reference :default "/Game/TT_269/Core/Inputs/InputActions/IA_Inventory.IA_Inventory"))
  ;[1 1 1] Inputs:
  ;;[1 1 1] Show inventory input:
  (:Started
    (CallFunction|ShowInventoryWidget)))

(event Input|EnhancedActionEvents|EnhancedInputActionIA_Attack
  (params (ActionValue :type Boolean) (ElapsedSeconds :type Float%20%28double-precision%29) (TriggeredSeconds :type Float%20%28double-precision%29) (InputAction :type Input%20Action%20Object%20Reference :default "/Game/TT_269/Core/Inputs/InputActions/IA_Attack.IA_Attack"))
  ;[1 1 1] Inputs:
  ;;[1 1 1] Attack input:
  (:Started
    (bind _currentweapon (Variables|Weapon|GetCurrentWeapon)
      (:then
        (Class|WeaponMain|Attack _currentweapon))
      (:else)))
  (:Completed
    (bind _currentweapon_2 (Variables|Weapon|GetCurrentWeapon)
      (:then
        (Class|WeaponMain|StopAttack _currentweapon_2))
      (:else))))

(event Input|EnhancedActionEvents|EnhancedInputActionIA_SlotWeapon_One
  (params (ActionValue :type Boolean) (ElapsedSeconds :type Float%20%28double-precision%29) (TriggeredSeconds :type Float%20%28double-precision%29) (InputAction :type Input%20Action%20Object%20Reference :default "/Game/TT_269/Core/Inputs/InputActions/IA_SlotWeapon_One.IA_SlotWeapon_One"))
  ;[1 1 1] Inputs:
  ;;[1 1 1] Set weapon slot First:
  (:Started
    (Weapon|SetCurrnetWeaponAmmoQuantity)
    (Class|WeaponInventoryComponent|SetCurrentWeaponInfobySlotType (Variables|Default|GetWeaponInventory) "First_Type" false)))

(event Input|EnhancedActionEvents|EnhancedInputActionIA_SlotWeapon_Two
  (params (ActionValue :type Boolean) (ElapsedSeconds :type Float%20%28double-precision%29) (TriggeredSeconds :type Float%20%28double-precision%29) (InputAction :type Input%20Action%20Object%20Reference :default "/Game/TT_269/Core/Inputs/InputActions/IA_SlotWeapon_Two.IA_SlotWeapon_Two"))
  ;[1 1 1] Inputs:
  ;;[1 1 1] Set weapon slot Second:
  (:Started
    (Weapon|SetCurrnetWeaponAmmoQuantity)
    (Class|WeaponInventoryComponent|SetCurrentWeaponInfobySlotType (Variables|Default|GetWeaponInventory) "Second_Type" false)))

(event Input|EnhancedActionEvents|EnhancedInputActionIA_Reload
  (params (ActionValue :type Boolean) (ElapsedSeconds :type Float%20%28double-precision%29) (TriggeredSeconds :type Float%20%28double-precision%29) (InputAction :type Input%20Action%20Object%20Reference :default "/Game/TT_269/Core/Inputs/InputActions/IA_Reload.IA_Reload"))
  ;[1 1 1] Inputs:
  ;;[1 1 1] Reload input:
  (:Started
    (Weapon|StartReload)))

(event Input|EnhancedActionEvents|EnhancedInputActionIA_UseFirstAidKit
  (params (ActionValue :type Boolean) (ElapsedSeconds :type Float%20%28double-precision%29) (TriggeredSeconds :type Float%20%28double-precision%29) (InputAction :type Input%20Action%20Object%20Reference :default "/Game/TT_269/Core/Inputs/InputActions/IA_UseFirstAidKit.IA_UseFirstAidKit"))
  ;[1 1 1] Inputs:
  ;;[1 1 1] Use first aid kit input:
  (:Started
    (CallFunction|UseFirstAidKit)))

(event Input|EnhancedActionEvents|EnhancedInputActionIA_SaveGame
  (params (ActionValue :type Boolean) (ElapsedSeconds :type Float%20%28double-precision%29) (TriggeredSeconds :type Float%20%28double-precision%29) (InputAction :type Input%20Action%20Object%20Reference :default "/Game/TT_269/Core/Inputs/InputActions/IA_SaveGame.IA_SaveGame"))
  (bind _returnvalue (Subsystems|GetSaveGameSubsystem))
  ;[1 1 1] Inputs:
  ;;[1 1 1] Load/Save game inputs:
  (:Started
    (Class|SaveGameSubsystem|SaveGameObject _returnvalue (Class|SaveGameSubsystem|GetCurrentSaveGameSlot _returnvalue) (Class|SaveGameSubsystem|GetCurrentSaveGameObject _returnvalue))))

(event Input|EnhancedActionEvents|EnhancedInputActionIA_LoadGame
  (params (ActionValue :type Boolean) (ElapsedSeconds :type Float%20%28double-precision%29) (TriggeredSeconds :type Float%20%28double-precision%29) (InputAction :type Input%20Action%20Object%20Reference :default "/Game/TT_269/Core/Inputs/InputActions/IA_LoadGame.IA_LoadGame"))
  (bind _returnvalue (Subsystems|GetSaveGameSubsystem))
  ;[1 1 1] Inputs:
  ;;[1 1 1] Load/Save game inputs:
  (:Started
    (bind (_savegameobject _returnvalue_2) (Class|SaveGameSubsystem|LoadSaveGame _returnvalue "Test"))
    (if _returnvalue_2
      (bind _assave_game_main (Utilities|Casting|CastToSaveGameMain _savegameobject))
      (Class|SaveGameSubsystem|SetCurrentSaveGameObject _returnvalue "Test" _assave_game_main))))

(event EventBeginPlay
  (|CallParentFunction)
  (Utilities|FlowControl|Sequence
    (:then_1
      ;[1 1 1] Bind update weapon slot:
      (EventDispatchers|BindEventtoOnUpdateCurrentWeaponSlot (Variables|Default|GetWeaponInventory) (EventDispatchers|CreateEvent :!event UpdateCurrentWeaponSlot)))))

(event EventPossessed
  (params (NewController :type Controller%20Object%20Reference))
  (|CallParentFunction NewController)
  (Variables|Default|GetPlayerController
    (:then
      (Utilities|FlowControl|Sequence
        (:then_1
          ;[1 1 1] Set input mapping:
          (Class|PlayerControllerMain|SetInputMapping (Variables|Default|GetPlayerController) (Variables|Character|GetInputMapping)))
        (:then_2
          ;[1 1 1] Get HUD:
          (bind _asbp_hud_main (Utilities|Casting|CastToBP_HUD_Main (HUD|GetHUD (Variables|Default|GetPlayerController))))
          (Variables|Default|SetHUD _asbp_hud_main)
          ;[1 1 1] Show widgets:
          (bind _hud (Variables|Default|GetHUD)
            (:then
              (Default|ShowWeaponsInfoWidget _hud true)
              (Default|ShowPlayerHealthWidget _hud true))
            (:else)))))
    (:else)))

(fn ConstructionScript)

(fn ShowInventoryWidget
  (bind _hud (Variables|Default|GetHUD)
    (:then
      (Default|ShowInventoryWidget _hud (not (Default|IsShowInventoryWidget _hud))))
    (:else)))

(fn SpawnWeapon
  (params (WeaponActorInfo :type Weapon%20Actor%20Info%20Structure%20%28by%20ref%29))
  (bind _self self)
  (bind (_displayname _weaponclass _weaponslottype _pickupmesh _attachsocketname _maxammo _currentammo _characteranimation _weapondamageinfo _itemquantity _maxitemquantity _itemtype _itemname) (Utilities|Struct|BreakWeaponActorInfo WeaponActorInfo))
  (Utilities|FlowControl|Sequence
    (:then_0
      (bind _currentweapon (Variables|Weapon|GetCurrentWeapon)
        (:then
          (Actor|DestroyActor _currentweapon)
          (Default|CallOnUpdateCharacterAnimation))
        (:else)))
    (:then_1
      (bind _returnvalue (Game|SpawnActorfromClass _weaponclass (Transformation|GetSocketTransform (Variables|Character|GetMesh) _attachsocketname "RTS_World") "AlwaysSpawn" "MultiplyWithRoot" _self _itemname WeaponActorInfo _self))
      (Variables|Weapon|SetCurrentWeapon _returnvalue)
      (Variables|Weapon|GetCurrentWeapon
        (:then
          (Default|CallOnUpdateCharacterAnimation _characteranimation)
          (EventDispatchers|BindEventtoOnWeaponFireStart (Variables|Weapon|GetCurrentWeapon) (EventDispatchers|CreateEvent :!event Custom|PlayFireMontage_Event))
          (EventDispatchers|BindEventtoOnNeededReload (Variables|Weapon|GetCurrentWeapon) (EventDispatchers|CreateEvent :!event StartReload))
          (Transformation|AttachComponentToComponent (Variables|Weapon|GetCurrentWeapon) (Variables|Character|GetMesh) _attachsocketname "KeepWorld" "KeepWorld" "KeepWorld" true)
          (Default|CallOnSpawnWeapon (Variables|Weapon|GetCurrentWeapon)))
        (:else)))))

(fn UpdateCurrentWeaponSlot
  (params (SlotType :type EWeaponSlotType%20Enum :default "None_Type") (WeaponActorInfo :type Weapon%20Actor%20Info%20Structure))
  (Weapon|SpawnWeapon WeaponActorInfo))

(fn StartReload
  (bind _currentweapon (Variables|Weapon|GetCurrentWeapon))
  (bind _currentweapon_2 (Variables|Weapon|GetCurrentWeapon))
  (bind _outinfo (Class|WeaponMain|GetWeaponActorInfo _currentweapon_2))
  (bind _characteranimation (Utilities|Struct|BreakWeaponActorInfo _outinfo))
  (bind _reloadanimmontage (Utilities|Struct|BreakCharacterAnimationInfo _characteranimation))
  (Variables|Weapon|GetCurrentWeapon
    (:then
      (if (not (Variables|Weapon|GetbIsReload))
        (if (not (== (Class|WeaponMain|GetMaxAmmoQuantity _currentweapon) (Class|WeaponMain|GetCurrentAmmoQuantity _currentweapon)))
          (Utilities|IsValid _reloadanimmontage
            (:Is%20Valid
              ;[1 1 1] Is Have item?
              (if (> (.ReturnValue (Class|InventoryComponent|IsHaveItembyName (Variables|Default|GetWeaponInventory) (.ItemName (Utilities|Struct|BreakWeaponActorInfo (Variables|/Script/TT_269.WeaponMain|GetWeaponActorInfo (Variables|Weapon|GetCurrentWeapon)))))) -1)
                (CallFunction|PlayReloadAnimEvent _reloadanimmontage)
                (Variables|Weapon|SetbIsReload true)))
            (:Is%20Not%20Valid
              (Weapon|Reload))))))
    (:else)))

(fn Reload
  (bind _currentweapon (Variables|Weapon|GetCurrentWeapon))
  (bind _currentweapon_2 (Variables|Weapon|GetCurrentWeapon))
  (bind _weaponinventory (Variables|Default|GetWeaponInventory))
  (bind _weaponactorinfo (Variables|/Script/TT_269.WeaponMain|GetWeaponActorInfo _currentweapon))
  (bind _itemname (Utilities|Struct|BreakWeaponActorInfo _weaponactorinfo))
  (bind _itemactorinfo (Utilities|Struct|MakeItemActorInfo "Ammo_Type" _itemname))
  (bind (_outinfo _returnvalue) (Class|InventoryComponent|GetItemInventoryInfo _weaponinventory _itemactorinfo))
  ;[1 1 1] Get ammo item from WeaponInventory:
  (Variables|Weapon|SetbIsReload false)
  (LocalVariables|SetItemIndex_Local _returnvalue)
  (LocalVariables|SetItemInfo_Local _outinfo)
  ;[1 1 1] Is find?
  (if (> (LocalVariables|GetItemIndex_Local) -1)
    (LocalVariables|SetNeededAmmoQuantity_Local (- (Class|WeaponMain|GetMaxAmmoQuantity _currentweapon_2) (Class|WeaponMain|GetCurrentAmmoQuantity _currentweapon_2)))
    (if (>= (LocalVariables|GetNeededAmmoQuantity_Local) (.ItemQuantity (Utilities|Struct|BreakInventorySlotInfo (LocalVariables|GetItemInfo_Local))))
      (Class|WeaponMain|AddAmmoQuantity (Variables|Weapon|GetCurrentWeapon) (.ItemQuantity (Utilities|Struct|BreakInventorySlotInfo (LocalVariables|GetItemInfo_Local))))
      (Class|InventoryComponent|ChangeInventorySlot (Variables|Default|GetWeaponInventory) (LocalVariables|GetItemIndex_Local) (Utilities|Struct|MakeInventorySlotInfo 0 0 "None_Type" "None"))
      (else
        (Class|WeaponMain|AddAmmoQuantity (Variables|Weapon|GetCurrentWeapon) (LocalVariables|GetNeededAmmoQuantity_Local))
        (Utilities|Struct|SetmembersinInventorySlotInfo (LocalVariables|GetItemInfo_Local) (- (.ItemQuantity (Utilities|Struct|BreakInventorySlotInfo (LocalVariables|GetItemInfo_Local))) (LocalVariables|GetNeededAmmoQuantity_Local)))
        (Class|InventoryComponent|ChangeInventorySlot (Variables|Default|GetWeaponInventory) (LocalVariables|GetItemIndex_Local) (LocalVariables|GetItemInfo_Local))))))

(fn UseFirstAidKit
  (LocalVariables|SetItemIndex_Local (.ReturnValue (Class|InventoryComponent|GetItemInventoryInfo (Variables|Default|GetWeaponInventory) (Utilities|Struct|MakeItemActorInfo "Other_Type" "FirstAidKit"))))
  (if (> (LocalVariables|GetItemIndex_Local) -1)
    (Class|HealthComponent|RestoreHealth (Variables|Default|GetHealthMain))
    (Class|InventoryComponent|ChangeInventorySlot (Variables|Default|GetWeaponInventory) (LocalVariables|GetItemIndex_Local) (Utilities|Struct|MakeInventorySlotInfo 0 0 "None_Type" "None"))))

(fn LoadPlayerInformation
  (params (PlayerCharacterSaveInfo :type Player%20Character%20Save%20Info%20Structure%20%28by%20ref%29))
  (bind (_health _inventoryinfo _weaponsinfo) (Utilities|Struct|BreakPlayerCharacterSaveInfo PlayerCharacterSaveInfo))
  (bind _weaponinventory (Variables|Default|GetWeaponInventory))
  (Utilities|FlowControl|Sequence
    (:then_0
      (Class|HealthComponent|SetCurrentHealth (Variables|Default|GetHealthMain) _health))
    (:then_1
      (Class|InventoryComponent|LoadInventoryInfo _weaponinventory _inventoryinfo)
      (Class|WeaponInventoryComponent|LoadWeaponsInfo _weaponinventory _weaponsinfo))))

(fn SetCurrnetWeaponAmmoQuantity
  (bind _currentweapon (Variables|Weapon|GetCurrentWeapon)
    (:then
      (Class|WeaponInventoryComponent|UpdateCurrentWeaponAmmoQuantity (Variables|Default|GetWeaponInventory) (.CurrentAmmo (Utilities|Struct|BreakWeaponActorInfo (Class|WeaponMain|GetWeaponActorInfo _currentweapon))))
      (return))
    (:else
      (return))))
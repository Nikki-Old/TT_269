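; Weapon pickup actor that puts an item into the interacting actor's inventory.
; The construction script synchronously loads the weapon DataTable and sets the pickup mesh from the row matching the item data asset's name.
; Interaction functions toggle the prompt widget and report whether the pickup is still unused.
; StartInteract adds the item and quantity to the instigator's InventoryComponent, then marks itself used and destroys itself only on success.
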(event EventBeginPlay)

(fn ConstructionScript
  (bind _returnvalue (Utilities|LoadAssetBlocking (Variables|Default|GetWeaponTable)))
  (bind _asdata_table (Utilities|Casting|CastToDataTable _returnvalue))
  (bind _outinfo (Class|ItemDataAsset|GetItemInfo (Variables|Default|GetItemDataAsset)))
  (bind _returnvalue_2 (Utilities|GetDataTableRow _asdata_table (.ItemName (Utilities|Struct|BreakItemActorInfo _outinfo)))
    (:then
      (bind _output_get (LocalVariables|SetWeaponActorInfo_Local _returnvalue_2))
      (Components|StaticMesh|SetStaticMesh (Variables|Default|GetMesh) (.PickUpMesh (Utilities|Struct|BreakWeaponActorInfo _output_get))))))

(fn ShowCanInteract
  (if (not (Variables|Default|GetbIsShow))
    (Variables|Default|SetbIsShow true)
    (bind _bp_widget_interact (Variables|Default|GetBP_Widget_Interact)
      (:then
        (Default|ShowInteractWidget _bp_widget_interact true)
        (return true))
      (:else))))

(fn IsCanInteract
  (return (not (Variables|Default|GetbIsUse))))

(fn StartInteract
  (params (InteractInstigator :type Actor%20Object%20Reference))
  (Variables|Default|GetItemDataAsset
    (:then
      (LocalVariables|SetInventoryComp_Local (Actor|GetComponentbyClass InteractInstigator "/Script/TT_269.InventoryComponent"))
      (bind _inventorycomp_local (LocalVariables|GetInventoryComp_Local)
        (:then
          (bind _returnvalue (Class|InventoryComponent|AddItemInfo _inventorycomp_local (Variables|/Script/TT_269.ItemDataAsset|GetItemInfo (Variables|Default|GetItemDataAsset)) (Variables|PickUp|GetQuantity)))
          (if _returnvalue
            (Variables|Default|SetbIsUse true)
            (Actor|DestroyActor)
            (return true)
            (else
              (return false))))
        (:else
          _)))
    (:else
      _))
  (return false))

(fn UnShowCanInteract
  (if (not (Variables|Default|GetbIsUse))
    (Variables|Default|SetbIsShow false)
    (bind _bp_widget_interact (Variables|Default|GetBP_Widget_Interact)
      (:then
        (Default|ShowInteractWidget _bp_widget_interact false)
        (return true))
      (:else))))
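; BP_PickUp_Test is a test pickup actor that exposes interaction functions but has no pickup behavior.
; ShowCanInteract and UnShowCanInteract toggle the prompt on its BPWidgetInteract and report success.
; IsCanInteract always returns true, while StartInteract ignores the instigator and returns false.
; BeginPlay and the construction script are empty.
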(event EventBeginPlay)

(fn ConstructionScript)

(fn ShowCanInteract
  (Default|ShowInteractWidget (Variables|Default|GetBP_Widget_Interact) true)
  (return true))

(fn IsCanInteract
  (return true))

(fn StartInteract
  (params (InteractInstigator :type Actor%20Object%20Reference))
  (return false))

(fn UnShowCanInteract
  (Default|ShowInteractWidget (Variables|Default|GetBP_Widget_Interact) false)
  (return true))
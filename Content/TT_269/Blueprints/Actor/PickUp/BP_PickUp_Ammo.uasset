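; Ammo pickup actor that adds its item to the interacting actor's inventory component and destroys itself on success.
; The construction script takes item info from the data asset, looks up the matching ammo table row by item name and applies that row's mesh.
; Interaction functions toggle a prompt widget and report the pickup as interactable until it is used.
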(event EventBeginPlay
  (|CallParentFunction))

(fn ConstructionScript
  (CallFunction|Initialize))

(fn IsCanInteract
  (return (not (Variables|Default|GetbIsUse))))

(fn ShowCanInteract
  (if (not (Variables|Default|GetbIsShow))
    (Variables|Default|SetbIsShow true)
    (bind _bp_widget_interact (Variables|Default|GetBP_Widget_Interact)
      (:then
        (Default|ShowInteractWidget _bp_widget_interact true)
        (return true))
      (:else))))

(fn StartInteract
  (params (InteractInstigator :type Actor%20Object%20Reference))
  (Variables|Default|GetItemDataAsset
    (:then
      (LocalVariables|SetInventoryComp_Local (Actor|GetComponentbyClass InteractInstigator "/Script/TT_269.InventoryComponent"))
      (bind _inventorycomp_local (LocalVariables|GetInventoryComp_Local)
        (:then
          (bind _returnvalue (Class|InventoryComponent|AddItemInfo _inventorycomp_local (Variables|Default|GetItemActorInfo) (Variables|PickUp|GetQuantity)))
          (if _returnvalue
            (Variables|Default|SetbIsUse true)
            (Actor|DestroyActor)
            (return true)
            (else
              (return false))))
        (:else
          _)))
    (:else
      _))
  (return false))

(fn UnShowCanInteract
  (if (not (Variables|Default|GetbIsUse))
    (Variables|Default|SetbIsShow false)
    (bind _bp_widget_interact (Variables|Default|GetBP_Widget_Interact)
      (:then
        (Default|ShowInteractWidget _bp_widget_interact false)
        (return true))
      (:else))))

(fn Initialize
  (if (Variables|Default|GetbIsInitialized)
    _
    (else
      (bind _returnvalue (Utilities|LoadAssetBlocking (Variables|Default|GetAmmoTable_Local)))
      (bind _asdata_table (Utilities|Casting|CastToDataTable _returnvalue))
      (Variables|Default|SetItemActorInfo (Class|ItemDataAsset|GetItemInfo (Variables|Default|GetItemDataAsset)))
      (bind _returnvalue_2 (Utilities|GetDataTableRow _asdata_table (.ItemName (Utilities|Struct|BreakItemActorInfo (Variables|Default|GetItemActorInfo))))
        (:then
          (Variables|Default|SetAmmoInfo _returnvalue_2)
          (Variables|Default|SetbIsInitialized true)))))
  (Components|StaticMesh|SetStaticMesh (Variables|Default|GetMesh) (.Mesh (Utilities|Struct|BreakAmmoActorInfo (Variables|Default|GetAmmoInfo)))))
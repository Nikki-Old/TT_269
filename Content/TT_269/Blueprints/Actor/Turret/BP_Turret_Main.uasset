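; BP_Turret_Main is a turret actor that starts shooting at pawns it sees or at whoever damages it.
; On BeginPlay it runs the parent logic, then connects its Health component to the health bar widget.
; A sighting or health change calls StartShootToTarget with that pawn or last damage causer, then deactivates PawnSensing.
; The Health component's death event destroys the actor.
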(event OnSeePawn(PawnSensing)
  (params (Pawn :type Pawn%20Object%20Reference))
  (Class|TurretMain|StartShoottoTarget Pawn)
  (Components|Activation|Deactivate (Variables|Default|GetPawnSensing)))

(event OnDead(Health)
  (params (Owner :type Actor%20Object%20Reference) (LastDamageCauser :type Actor%20Object%20Reference))
  (Actor|DestroyActor))

(event OnChangeHealth(Health)
  (params (Owner :type Actor%20Object%20Reference) (CurrentHealth :type Float%20%28single-precision%29) (Change :type Float%20%28single-precision%29))
  (Class|TurretMain|StartShoottoTarget (Class|HealthComponent|GetLastDamageCauser (Variables|Default|GetHealth)))
  (Components|Activation|Deactivate (Variables|Default|GetPawnSensing)))

(event EventBeginPlay
  (|CallParentFunction)
  (Utilities|FlowControl|Sequence
    (:then_0
      ;[1 1 1] Create between Health component and HealthBar:
      (bind _aswbp_heatlh_bar (Utilities|Casting|CastToWBP_HeatlhBar (UserInterface|GetWidget (Variables|Default|GetHealthWidget))))
      (Class|HealthBarWidget|CreateConnectwithHealthComponent _aswbp_heatlh_bar (Variables|Default|GetHealth)))))

(fn ConstructionScript)
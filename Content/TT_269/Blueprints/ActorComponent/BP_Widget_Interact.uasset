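; BP_Widget_Interact is a widget component Blueprint that shows or hides an interaction widget.
; On BeginPlay it calls the parent implementation, then requests the hidden state.
; ShowInteractWidget compares the requested state with IsShow and, only on a change, stores it and sets the component's widget to Visible or Collapsed.
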(event EventBeginPlay
  (|CallParentFunction)
  (CallFunction|ShowInteractWidget false))

(event EventTick
  (params (DeltaSeconds :type Float%20%28single-precision%29)))

(fn ShowInteractWidget
  (params (bIsNewShow :type Boolean))
  (bind _self self)
  (bind _returnvalue (UserInterface|GetWidget _self))
  (if (!= bIsNewShow (Variables|Default|GetbIsShow))
    (bind _output_get (Variables|Default|SetbIsShow bIsNewShow))
    (if _output_get
      (Widget|SetVisibility _returnvalue "Visible")
      (else
        (Widget|SetVisibility _returnvalue "Collapsed")))))